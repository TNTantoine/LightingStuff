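; BP_Light_Path moves two referenced light actors, Light and DFLight, plus a sphere component along a looping spline.
; Tick advances DistanceAlongSpline by Speed and delta time, resets it to zero at the spline's end, and repositions all three in world space.
; The construction script and BeginPlay also place them at the current distance.
; Pressing Enter toggles the visibility of both lights, leaving the sphere untouched.
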(event EventBeginPlay
  (bind _distancealongspline (Variables|Default|GetDistanceAlongSpline))
  (bind _spline (Variables|Default|GetSpline))
  (bind _returnvalue (Spline|GetLocationatDistanceAlongSpline _spline _distancealongspline "World"))
  (Transformation|SetActorLocation (Variables|Default|GetDF_Light) _returnvalue false false)
  (Transformation|SetActorLocation (Variables|Default|GetLight) _returnvalue false false)
  (Transformation|SetWorldLocation (Variables|Default|GetSphere) _returnvalue false false))

(event EventTick
  (params (DeltaSeconds :type Float%20%28single-precision%29))
  (if (< (+ (* DeltaSeconds (Variables|Default|GetSpeed)) (Variables|Default|GetDistanceAlongSpline)) (Spline|GetSplineLength (Variables|Default|GetSpline)))
    (Variables|Default|SetDistanceAlongSpline (+ (* DeltaSeconds (Variables|Default|GetSpeed)) (Variables|Default|GetDistanceAlongSpline)))
    (else
      (Variables|Default|SetDistanceAlongSpline 0.0)))
  (Transformation|SetActorLocation (Variables|Default|GetDF_Light) (Spline|GetLocationatDistanceAlongSpline (Variables|Default|GetSpline) (Variables|Default|GetDistanceAlongSpline) "World") false false)
  (Transformation|SetActorLocation (Variables|Default|GetLight) (Spline|GetLocationatDistanceAlongSpline (Variables|Default|GetSpline) (Variables|Default|GetDistanceAlongSpline) "World") false false)
  (Transformation|SetWorldLocation (Variables|Default|GetSphere) (Spline|GetLocationatDistanceAlongSpline (Variables|Default|GetSpline) (Variables|Default|GetDistanceAlongSpline) "World") false false))

(event Input|KeyboardEvents|Enter
  (params (Key :type Key%20Structure))
  (:Pressed
    (Rendering|ToggleVisibility (Variables|/Script/Engine.Light|GetLightComponent (Variables|Default|GetLight)) false)))

(fn ConstructionScript
  (bind _distancealongspline (Variables|Default|GetDistanceAlongSpline))
  (bind _spline (Variables|Default|GetSpline))
  (bind _returnvalue (Spline|GetLocationatDistanceAlongSpline _spline _distancealongspline "World"))
  (Transformation|SetActorLocation (Variables|Default|GetLight) _returnvalue false false)
  (Transformation|SetActorLocation (Variables|Default|GetDF_Light) _returnvalue false false)
  (Transformation|SetWorldLocation (Variables|Default|GetSphere) _returnvalue false false))